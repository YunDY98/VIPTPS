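; Shooting game HUD Blueprint that relays the player's HP, magazine and ammo updates to the HudWidget.
; Each update event casts the widget reference and calls its matching setter; HP and magazine updates are dropped if the cast fails.
; Ammo is cached in TempAmmo, and FirstUpdate retries on a short function-name timer until the widget is valid, so the initial value still shows.
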(event `self.OnUpdateMyHp`
  (params (CurrentHp :type "Float (single-precision)") (MaxHp :type "Float (single-precision)"))
  (bind _ashud_widget (cast `/Game/ShootingGame/Widget/HudWidget` (`self.HudWidget`)))
  (`/Game/ShootingGame/Widget/HudWidget.SetHp` _ashud_widget CurrentHp MaxHp))

(event `self.OnUpdateMyMag`
  (params (Mag :type Integer))
  (bind _ashud_widget (cast `/Game/ShootingGame/Widget/HudWidget` (`self.HudWidget`)))
  (`/Game/ShootingGame/Widget/HudWidget.SetMag` _ashud_widget Mag))

(event `self.OnUpdateMyAmmo`
  (params (Ammo :type Integer))
  (set `self.TempAmmo` Ammo)
  (bind _ashud_widget (cast `/Game/ShootingGame/Widget/HudWidget` (`self.HudWidget`))
    (:`then`
      (`/Game/ShootingGame/Widget/HudWidget.SetAmmo` _ashud_widget Ammo))
    (:`CastFailed`
      (`self.FirstUpdate`))))

(fn `FirstUpdate`
  (bind _ashud_widget (cast `/Game/ShootingGame/Widget/HudWidget` (`self.HudWidget`))
    (:`then`
      (`/Game/ShootingGame/Widget/HudWidget.SetAmmo` _ashud_widget (`self.TempAmmo`)))
    (:`CastFailed`
      (`KismetSystemLibrary.K2_SetTimer` null "FirstUpdate" 0.1))))

(fn `UserConstructionScript`)