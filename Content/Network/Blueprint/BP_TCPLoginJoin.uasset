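; BP_TCPLoginJoin is a TCP client that handles login and join requests against a local server.
; On BeginPlay it connects to a hardcoded localhost port and tracks the connection ID.
; Send functions transmit the ID with a "0" prefix, a join ID with "1", and the password unprefixed, resetting the socket on failure.
; Incoming messages are read as strings into CheckID and printed.
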(event `self.ReceiveBeginPlay`
  (`self.Connect` "127.0.0.1" 5959 (delegate `TCPDisconnected`) (delegate `TCPConnected`) (delegate `OnRecvMessage`)))

(event `TCPDisconnected`
  (params (ConnectionId :type Integer))
  (set `self.ServerSocket` -1))

(event `TCPConnected`
  (params (ConnectionId :type Integer))
  (set `self.ServerSocket` ConnectionId))

(event `OnRecvMessage`
  (params (ConnectionId :type Integer) (Message :type "Array of Byte (by ref)"))
  (bind _returnvalue (`self.Message_ReadString` Message (`KismetArrayLibrary.Array_Length` Message)))
  (bind _output_get (set `self.CheckID` _returnvalue))
  (`KismetSystemLibrary.PrintString` _output_get))

(fn `TCPID`
  (params (Message :type String))
  (bind _serversocket (`self.ServerSocket`))
  (bind _returnvalue (`self.SendData` _serversocket (`self.Conv_StringToBytes` (`KismetStringLibrary.Concat_StrStr` "0" Message))))
  (if (not _returnvalue)
    (`self.TCPDisconnected` _serversocket)
    (set `self.ServerSocket` 0)))

(fn `TCPJoin`
  (params (JoinID :type String))
  (bind _serversocket (`self.ServerSocket`))
  (bind _returnvalue (`self.SendData` _serversocket (`self.Conv_StringToBytes` (`KismetStringLibrary.Concat_StrStr` "1" JoinID))))
  (if (not _returnvalue)
    (`self.TCPDisconnected` _serversocket)
    (set `self.ServerSocket` 0)))

(fn `TCPPWD`
  (params (PWD :type String))
  (bind _returnvalue (`self.SendData` (`self.ServerSocket`) (`self.Conv_StringToBytes` PWD)))
  (if (not _returnvalue)
    (`self.TCPDisconnected` 0)
    (set `self.ServerSocket` 0)))

(fn `UserConstructionScript`)